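; Event display actor for an ATLAS visualisation that loads, draws and toggles jets, tracks and clusters.
; Previous/next (or F) changes EventID, then UpdateEvent destroys old Jet, Cluster and Track actors and calls GetEvent.
; On download it updates run/event text, then Tick ramps PercentLoad, redrawing through ShowClustersFunc and ShowTracksFunc for progressive loading.
; The Blueprint's own procedural-mesh ShowClusters/ShowTracks bodies are disconnected; auto-reload toggling schedules a one-shot UpdateEvent timer.
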(event EventToggleTracks
  (Rendering|ToggleVisibility (Variables|Default|GetmeshX) false)
  (Rendering|ToggleVisibility (Variables|Default|GetmeshY) false))

(event EventToggleJets
  (CallFunction|LToggleJets))

(event EventToggleClusters
  (Rendering|ToggleVisibility (Variables|Default|GetmeshCluster) false))

(event EventLoadPrevious
  (CallFunction|LLoadPrevious))

(event EventLoadNext
  (CallFunction|LLoadNext))

(event EventTick
  (params (DeltaSeconds :type Float%20%28single-precision%29))
  (if (< (Variables|Default|GetpercentLoad) 1.0)
    (Variables|Default|SetpercentLoad (+ (Variables|Default|GetpercentLoad) 0.01))
    (CallFunction|DrawEvent)))

(event EventOnEventDownloaded
  (CallFunction|DrawScreen)
  (Variables|Default|SetpercentLoad 0.0)
  (CallFunction|DrawEvent))

(event EventToggleAutoLoad
  (Variables|Default|SetEventState (Utilities|Struct|MakeEventState (.ShowTracks (Utilities|Struct|BreakEventState (Variables|Default|GetEventState))) (.ShowJets (Utilities|Struct|BreakEventState (Variables|Default|GetEventState))) (.ShowClusters (Utilities|Struct|BreakEventState (Variables|Default|GetEventState))) (not (.AutoReload (Utilities|Struct|BreakEventState (Variables|Default|GetEventState)))) (.ChangeToPreviousEvent (Utilities|Struct|BreakEventState (Variables|Default|GetEventState))) (.ChangeToNextEvent (Utilities|Struct|BreakEventState (Variables|Default|GetEventState)))))
  (Development|PrintString "Auto RELOAD is set to " false)
  (Development|PrintString (Utilities|String|ToString(Boolean) (not (.AutoReload (Utilities|Struct|BreakEventState (Variables|Default|GetEventState))))) false)
  (Utilities|Time|SetTimerbyFunctionName 0 "UpdateEvent" 5.0))

(event Input|KeyboardEvents|F
  (params (Key :type Key%20Structure))
  (:Pressed
    (Development|SetHiddeninGame (Variables|Default|GetInfoScreen) false true)
    (CallFunction|LLoadNext)))

(fn ConstructionScript
  (bind _asatlasgame_instance (Utilities|Casting|CastToATLASGameInstance (Game|GetGameInstance)))
  (Variables|Default|SetCurrentSettings (Variables|/Game/Maps/ATLASGameInstance.ATLASGameInstance_C|GetSaveData _asatlasgame_instance)))

(fn ShowClusters)

(fn LToggleJets
  (Development|PrintString "Toggle Jets!" false)
  (bind _outactors (Actor|GetAllActorsOfClass "/Script/ATLASrift.Jet"))
  (for _array_element _outactors
    (Rendering|ToggleVisibility (Utilities|Array|Get(acopy) (Actor|GetComponentsByClass _array_element "/Script/Engine.StaticMeshComponent")) false)))

(fn LLoadPrevious
  (Development|PrintString "Loading previous !")
  (Variables|Default|SetEventState (Utilities|Struct|MakeEventState (.ShowTracks (Utilities|Struct|BreakEventState (Variables|Default|GetEventState))) (.ShowJets (Utilities|Struct|BreakEventState (Variables|Default|GetEventState))) (.ShowClusters (Utilities|Struct|BreakEventState (Variables|Default|GetEventState))) (.AutoReload (Utilities|Struct|BreakEventState (Variables|Default|GetEventState))) true (.ChangeToNextEvent (Utilities|Struct|BreakEventState (Variables|Default|GetEventState)))))
  (Math|Integer|DecrementInt (Variables|Default|GeteventID)
    (:%20%20
      (CallFunction|UpdateEvent))))

(fn LLoadNext
  (Development|PrintString "Loading Next !")
  (Variables|Default|SetEventState (Utilities|Struct|MakeEventState (.ShowTracks (Utilities|Struct|BreakEventState (Variables|Default|GetEventState))) (.ShowJets (Utilities|Struct|BreakEventState (Variables|Default|GetEventState))) (.ShowClusters (Utilities|Struct|BreakEventState (Variables|Default|GetEventState))) (.AutoReload (Utilities|Struct|BreakEventState (Variables|Default|GetEventState))) (.ChangeToPreviousEvent (Utilities|Struct|BreakEventState (Variables|Default|GetEventState))) true))
  (Math|Integer|IncrementInt (Variables|Default|GeteventID)
    (:%20%20
      (CallFunction|UpdateEvent))))

(fn DrawEvent
  (bind _eventstate (Variables|Default|GetEventState))
  (bind (_showtracks _showjets _showclusters) (Utilities|Struct|BreakEventState _eventstate))
  (if _showclusters
    (Class|Event|ShowClustersFunc))
  (if _showtracks
    (Class|Event|ShowTracksFunc)))

(fn UpdateEvent
  (CallFunction|ClearPreviousEvent)
  (Class|Event|GetEvent)
  (Audio|PlaySoundatLocation "/Game/Audio/clong_Cue.clong_Cue" "0, 0, 0" "0, 0, 0" 1.0 0.2))

(fn ClearPreviousEvent
  (Development|PrintString "Removing previous event" false)
  (bind _outactors (Actor|GetAllActorsOfClass "/Script/ATLASrift.Jet"))
  (for _array_element _outactors
    (Actor|DestroyActor _array_element))
  (bind _outactors_2 (Actor|GetAllActorsOfClass "/Script/ATLASrift.Cluster"))
  (for _array_element_2 _outactors_2
    (Actor|DestroyActor _array_element_2))
  (bind _outactors_3 (Actor|GetAllActorsOfClass "/Script/ATLASrift.Track"))
  (for _array_element_3 _outactors_3
    (Actor|DestroyActor _array_element_3)))

(fn ShowTracks)

(fn DrawScreen
  (bind _returnvalue (Class|Event|GetEventNr))
  (Rendering|Components|TextRender|SetText (Variables|Default|GetEventNumberDisplay) (Utilities|Text|ToText(Integer) _returnvalue false))
  (bind _returnvalue_2 (Class|Event|GetRunNr))
  (Rendering|Components|TextRender|SetText (Variables|Default|GetRunNumberDisplay) (Utilities|Text|ToText(Integer) _returnvalue_2 false)))