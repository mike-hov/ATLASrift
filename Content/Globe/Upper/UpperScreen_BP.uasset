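; Video screen actor, set up through Initialize, that plays a media source when something overlaps its trigger box.
; Initialize stores the media references, assigns the sound, shows a pause material and play sign, and scales the screen to the pause texture's aspect ratio.
; First overlap swaps in the media material and opens the source with debug prints.
; End overlap pauses via zero rate; re-entry resumes, detected by "MediaPlayer" in the material name.
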(event OnComponentBeginOverlap(TriggerBox)
  (params (OverlappedComponent :type Primitive%20Component%20Object%20Reference) (OtherActor :type Actor%20Object%20Reference) (OtherComp :type Primitive%20Component%20Object%20Reference) (OtherBodyIndex :type Integer) (bFromSweep :type Boolean) (SweepResult :type Hit%20Result%20Structure%20%28by%20ref%29))
  (bind _mediaplayermat (Variables|Default|GetMediaPlayerMat))
  (bind _video (Variables|Default|GetVideo))
  (bind _streamingmediaplayer (Variables|Default|GetStreamingMediaPlayer))
  (if (Utilities|String|Contains (Utilities|GetDisplayName (Rendering|Material|GetMaterial (Variables|Default|GetScreen) 0)) "MediaPlayer")
    (Class|MediaPlayer|SetRate _streamingmediaplayer 1.0)
    (else
      (Development|SetHiddeninGame (Variables|Default|GetPlaySign) true false)
      (Rendering|Material|SetMaterial (Variables|Default|GetScreen) 0 _mediaplayermat)
      (bind _returnvalue (Media|MediaPlayer|OpenSource _streamingmediaplayer _video))
      (if _returnvalue
        (Development|PrintString "success")
        (Development|PrintString (Utilities|GetDisplayName _streamingmediaplayer) true true "(R=0.000000,G=0.660000,B=1.000000,A=1.000000)" 5.0)
        (Development|PrintString (Utilities|GetDisplayName _video) true true "(R=0.000000,G=0.660000,B=1.000000,A=1.000000)" 5.0)
        (Development|PrintString (Utilities|GetDisplayName _mediaplayermat) true true "(R=0.000000,G=0.660000,B=1.000000,A=1.000000)" 5.0)
        (Development|PrintString (Utilities|GetDisplayName (Variables|Default|GetSound)) true true "(R=0.000000,G=0.660000,B=1.000000,A=1.000000)" 5.0)
        (else
          (Development|PrintString "media source not opened"))))))

(event OnComponentEndOverlap(TriggerBox)
  (params (OverlappedComponent :type Primitive%20Component%20Object%20Reference) (OtherActor :type Actor%20Object%20Reference) (OtherComp :type Primitive%20Component%20Object%20Reference) (OtherBodyIndex :type Integer))
  (Class|MediaPlayer|SetRate (Variables|Default|GetStreamingMediaPlayer) 0.0))

(event EventBeginPlay)

(event Collision|EventActorBeginOverlap
  (params (OtherActor :type Actor%20Object%20Reference)))

(event EventTick
  (params (DeltaSeconds :type Float%20%28single-precision%29)))

(fn ConstructionScript)

(fn Initialize
  (params (Video :type Stream%20Media%20Source%20Object%20Reference) (MediaPlayer :type Media%20Player%20Object%20Reference) (MediaPlayerMat :type Material%20Object%20Reference) (MediaPlayerSound :type Media%20Sound%20Wave%20Object%20Reference) (PauseMaterial :type Material%20Object%20Reference) (PauseTexture :type Texture%202D%20Object%20Reference))
  (Variables|Default|SetVideo Video)
  (Variables|Default|SetStreamingMediaPlayer MediaPlayer)
  (Variables|Default|SetMediaPlayerMat MediaPlayerMat)
  (Audio|Components|Audio|SetSound (Variables|Default|GetSound) MediaPlayerSound)
  (Rendering|Material|SetMaterial (Variables|Default|GetScreen) 0 PauseMaterial)
  (Transformation|SetWorldScale3D (Variables|Default|GetScreen) (Math|Vector|MakeVector (* (/ (Math|Conversions|ToFloat(Integer) (Class|Texture2D|BlueprintGetSizeX PauseTexture)) (Math|Conversions|ToFloat(Integer) (Class|Texture2D|BlueprintGetSizeY PauseTexture))) 1.5) 1.5 1.0))
  (Development|SetHiddeninGame (Variables|Default|GetPlaySign) false false))