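; Poster actor for the globe that displays a configurable poster and can play an accompanying sound when the flying character is near.
; BeginPlay scales the poster plane from its ratio, applies its material, and reveals a Sign if a sound is assigned.
; A trigger box plays or resumes that audio on overlap with FlyingCharacter, matched by display name, and pauses it on any end overlap, swapping the Sign material to show state.
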(event OnComponentBeginOverlap(TriggerBox)
  (params (OverlappedComponent :type Primitive%20Component%20Object%20Reference) (OtherActor :type Actor%20Object%20Reference) (OtherComp :type Primitive%20Component%20Object%20Reference) (OtherBodyIndex :type Integer) (bFromSweep :type Boolean) (SweepResult :type Hit%20Result%20Structure%20%28by%20ref%29))
  ;[1 1 1] Start or unpause audio on overlap
  (if (Utilities|Enum|Equal(Enum) (Utilities|GetDisplayName OtherActor) "FlyingCharacter")
    (if (not (Variables|/Script/Engine.SceneComponent|GetbHiddenInGame (Variables|Default|GetSign)))
      (if (Audio|Components|Audio|IsPlaying (Variables|Default|GetAudio))
        (Class|AudioComponent|SetPaused (Variables|Default|GetAudio) false)
        (Variables|Default|SetPaused false)
        (else
          (Audio|Components|Audio|Play (Variables|Default|GetAudio) 0.0)))
      (Rendering|Material|SetMaterial (Variables|Default|GetSign) 0 (Variables|Default|GetisPlayingMat)))))

(event OnComponentEndOverlap(TriggerBox)
  (params (OverlappedComponent :type Primitive%20Component%20Object%20Reference) (OtherActor :type Actor%20Object%20Reference) (OtherComp :type Primitive%20Component%20Object%20Reference) (OtherBodyIndex :type Integer))
  ;[1 1 1] Pause audio when stop overlap
  (Class|AudioComponent|SetPaused (Variables|Default|GetAudio) true)
  (Variables|Default|SetPaused true)
  (Rendering|Material|SetMaterial (Variables|Default|GetSign) 0 (Variables|Default|GethasAudioMat)))

(event EventBeginPlay
  (CallFunction|SetAudioAsset)
  (CallFunction|SetPoster))

(fn ConstructionScript)

(fn SetAudioAsset
  (if (Utilities|IsValid (Variables|Default|GetSoundMat))
    (Audio|Components|Audio|SetSound (Variables|Default|GetAudio) (Variables|Default|GetSoundMat))
    (Development|SetHiddeninGame (Variables|Default|GetSign) false false)))

(fn SetPoster
  (bind _postermesh (Variables|Default|GetPosterMesh))
  (Transformation|SetWorldScale3D _postermesh (Math|Vector|MakeVector 1.2 (/ (Variables|Default|GetSurface) (Variables|Default|GetPosterRatio)) 0.0))
  (Rendering|Material|SetMaterial _postermesh 0 (Variables|Default|GetPosterMat))
  (Development|SetHiddeninGame (Variables|Default|GetPosterMesh) false false))